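; Actor that drives a humanoid skeletal mesh with Azure Kinect body tracking.
; On BeginPlay it creates and starts a Kinect device for its DeviceIndex and caches the AureKinectSkeletonToHumanoid anim blueprint of the referenced SkelertalMeshActor.
; Each tick it copies the first tracked skeleton into that anim blueprint while the device is open and tracking, then stops the device on EndPlay.
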(event EventBeginPlay
  (bind _returnvalue (Game|ConstructObjectfromClass "/Script/UnrealAzureKinect.AzureKinectDevice"))
  (Variables|Default|SetAzureKinect _returnvalue)
  (Variables|/Script/UnrealAzureKinect.AzureKinectDevice|SetDeviceIndex (Variables|Default|GetAzureKinect) (Variables|AzureKinect|GetDeviceIndex))
  (bind _returnvalue_2 (Class|AzureKinectDevice|Start (Variables|Default|GetAzureKinect)))
  (if _returnvalue_2
    (bind _asabp_aure_kinect_skeleton_to_humanoid (Utilities|Casting|CastToABP_AureKinectSkeletonToHumanoid (Components|SkeletalMesh|GetAnimInstance (Variables|/Script/Engine.SkeletalMeshActor|GetSkeletalMeshComponent (Variables|AzureKinect|GetSkelertalMeshActor)))))
    (Variables|Default|SetAnimBP _asabp_aure_kinect_skeleton_to_humanoid)))

(event EventTick
  (params (DeltaSeconds :type Float%20%28single-precision%29))
  (bind _azurekinect (Variables|Default|GetAzureKinect))
  (if (Math|Boolean|ANDBoolean (Class|AzureKinectDevice|IsOpen _azurekinect) (Class|AzureKinectDevice|HasTrackedSkeletons _azurekinect) (!= (Variables|Default|GetAnimBP) 0))
    (Variables|/UnrealAzureKinect/ABP_AureKinectSkeletonToHumanoid.ABP_AureKinectSkeletonToHumanoid_C|SetSkeleton (Variables|Default|GetAnimBP) (Class|AzureKinectDevice|GetSkeleton (Variables|Default|GetAzureKinect)))))

(event EventEndPlay
  (params (EndPlayReason :type EEndPlayReason%20Enum :default "Destroyed"))
  (Class|AzureKinectDevice|Stop (Variables|Default|GetAzureKinect)))

(fn ConstructionScript)